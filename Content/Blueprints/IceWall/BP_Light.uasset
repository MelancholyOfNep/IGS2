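; BP_Light is a switchable light with a SpotLight and a Bulb mesh.
; The construction script sets the spotlight's initial visibility from IsOn.
; ToggleLights flips IsOn, applies it to the spotlight along with LightColor, and calls SetMaterial on the bulb through a looping two-way MultiGate.
; The MultiGate alternates on each call without reading IsOn, so the bulb branch is independent of the starting state.
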(event EventToggleLights
  (bind _bulb (Variables|Default|GetBulb))
  (bind _output_get (Variables|Default|SetIs%20On? (not (Variables|Default|GetIs%20On?))))
  (Rendering|SetVisibility (Variables|Default|GetSpotLight) _output_get false)
  (Rendering|Components|Light|SetLightColor (Variables|Default|GetSpotLight) (Variables|Default|GetLight%20Color) true)
  (Utilities|FlowControl|MultiGate false true -1
    (:Out%200
      (Rendering|Material|SetMaterial _bulb 0 0))
    (:Out%201
      (Rendering|Material|SetMaterial _bulb 0 0))))

(fn ConstructionScript
  (Rendering|SetVisibility (Variables|Default|GetSpotLight) (Variables|Default|GetIs%20On?) false))