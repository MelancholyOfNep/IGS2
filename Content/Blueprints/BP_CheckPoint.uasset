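; BP_CheckPoint is a checkpoint actor that registers itself as the latest checkpoint when BP_Devvy enters its Box trigger.
; Any overlap plays a sound at the world origin, adds a WBP_Checkpoint widget to the viewport and switches the Cube to a warm glow material.
; Only then does it cast to BP_Devvy and store itself as LastCheckpoint on BP_ThirdPersonGameMode.
; Nothing guards against repeat triggers.
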(event OnComponentBeginOverlap(Box)
  (params (OverlappedComponent :type Primitive%20Component%20Object%20Reference) (OtherActor :type Actor%20Object%20Reference) (OtherComp :type Primitive%20Component%20Object%20Reference) (OtherBodyIndex :type Integer) (bFromSweep :type Boolean) (SweepResult :type Hit%20Result%20Structure%20%28by%20ref%29))
  (Audio|PlaySoundatLocation "/Game/Sounds/sound-alert-device-turn-on-turn-off-win-done-chakongaudio-174892.sound-alert-device-turn-on-turn-off-win-done-chakongaudio-174892" "0, 0, 0" "0, 0, 0" 1.0 1.0 0.0 0 0 0 0)
  (bind _returnvalue (UserInterface|CreateWidget "/Game/Widgets/WBP_Checkpoint.WBP_Checkpoint_C"))
  (UserInterface|Viewport|AddtoViewport _returnvalue 0)
  (Utilities|FlowControl|Sequence
    (:then_0
      (Rendering|Material|SetMaterial (Variables|Default|GetCube) 0 "/Game/Materials/LampGlowWarm.LampGlowWarm"))
    (:then_1
      (Utilities|Casting|CastToBP_Devvy OtherActor)
      (bind _asbp_third_person_game_mode (Utilities|Casting|CastToBP_ThirdPersonGameMode (Game|GetGameMode)))
      (Variables|/Game/ThirdPerson/Blueprints/BP_ThirdPersonGameMode.BP_ThirdPersonGameMode_C|Setlast%20Checkpoint _asbp_third_person_game_mode self))))

(fn ConstructionScript)