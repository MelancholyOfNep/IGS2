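; BP_ICEMonster is an ice monster actor that reacts only to fire damage.
; On AnyDamage, it checks whether the damage type is a child of DmgTypeBP_FireDamage.
; A match shows its Widget component and enables input from player 0 on the actor, then reverses both after a short delay.
; The graph defines no input handlers or health logic, and the construction script is empty.
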(event Game|Damage|EventAnyDamage
  (params (Damage :type Float%20%28single-precision%29) (DamageType :type Damage%20Type%20Object%20Reference) (InstigatedBy :type Controller%20Object%20Reference) (DamageCauser :type Actor%20Object%20Reference))
  (if (Utilities|ClassIsChildOf (Utilities|GetClass DamageType) "/Game/Blueprints/DamageTypes/DmgTypeBP_FireDamage.DmgTypeBP_FireDamage_C")
    (Rendering|SetVisibility (Variables|Default|GetWidget) true false)
    (Input|EnableInput (Game|GetPlayerController 0))
    (Utilities|FlowControl|Delay 4.0)
    (Rendering|SetVisibility (Variables|Default|GetWidget) false false)
    (Input|DisableInput (Game|GetPlayerController 0))))

(fn ConstructionScript)