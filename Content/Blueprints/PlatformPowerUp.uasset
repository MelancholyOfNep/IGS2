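; A pickup actor that grants the player's BP_Devvy pawn the platform power-up.
; Overlapping its Box shows a Widget component and enables player input on the actor; leaving hides the widget and disables input.
; On Interact it sets PlatformTime on the pawn, calls PickUpPowerMessage on PlatformVar, then destroys itself.
; The failed-cast branch redundantly repeats the same cast.
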(event OnComponentBeginOverlap(Box)
  (params (OverlappedComponent :type Primitive%20Component%20Object%20Reference) (OtherActor :type Actor%20Object%20Reference) (OtherComp :type Primitive%20Component%20Object%20Reference) (OtherBodyIndex :type Integer) (bFromSweep :type Boolean) (SweepResult :type Hit%20Result%20Structure%20%28by%20ref%29))
  ;[1 1 1] Widget
  (Rendering|SetVisibility (Variables|Default|GetWidget) true false)
  (Input|EnableInput (Game|GetPlayerController 0)))

(event OnComponentEndOverlap(Box)
  (params (OverlappedComponent :type Primitive%20Component%20Object%20Reference) (OtherActor :type Actor%20Object%20Reference) (OtherComp :type Primitive%20Component%20Object%20Reference) (OtherBodyIndex :type Integer))
  ;[1 1 1] Widget
  (Rendering|SetVisibility (Variables|Default|GetWidget) false false)
  (Input|DisableInput (Game|GetPlayerController 0)))

(event EventInteract
  (params (Character :type Character%20Object%20Reference))
  (bind _returnvalue (Game|Player|GetPlayerPawn 0))
  (bind _asbp_devvy (Utilities|Casting|CastToBP_Devvy _returnvalue)
    (:then
      (Variables|/Game/NewPlayerBP/Blueprints/BP_Devvy.BP_Devvy_C|SetPlatformTime? _asbp_devvy true))
    (:CastFailed
      (bind _asbp_devvy_2 (Utilities|Casting|CastToBP_Devvy _returnvalue))
      (Variables|/Game/NewPlayerBP/Blueprints/BP_Devvy.BP_Devvy_C|SetPlatformTime? _asbp_devvy_2 true)))
  (Class|PickUpPower|PickUpPower(Message) (Variables|Default|GetPlatformVar))
  (Actor|DestroyActor))

(fn ConstructionScript)