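; BP_NotePickupEnemy is a note pickup that the player character, BP_Devvy, can read while standing nearby.
; Entering its Box shows a Widget component and enables input on the actor.
; Interact then toggles the note by creating WBP_NoteElemental in the viewport or removing it.
; Leaving the Box puts the note down, hides the Widget and disables input.
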(event OnComponentBeginOverlap(Box)
  (params (OverlappedComponent :type Primitive%20Component%20Object%20Reference) (OtherActor :type Actor%20Object%20Reference) (OtherComp :type Primitive%20Component%20Object%20Reference) (OtherBodyIndex :type Integer) (bFromSweep :type Boolean) (SweepResult :type Hit%20Result%20Structure%20%28by%20ref%29))
  ;[1 1 1] Widget
  (Utilities|Casting|CastToBP_Devvy OtherActor)
  (Variables|Default|SetInReach? true)
  (Rendering|SetVisibility (Variables|Default|GetWidget) true false)
  (Input|EnableInput (Game|GetPlayerController 0)))

(event OnComponentEndOverlap(Box)
  (params (OverlappedComponent :type Primitive%20Component%20Object%20Reference) (OtherActor :type Actor%20Object%20Reference) (OtherComp :type Primitive%20Component%20Object%20Reference) (OtherBodyIndex :type Integer))
  ;[1 1 1] Widget
  (Utilities|Casting|CastToBP_Devvy OtherActor)
  (CallFunction|PutDownNote)
  (Variables|Default|SetInReach? false)
  (Rendering|SetVisibility (Variables|Default|GetWidget) false false)
  (Input|DisableInput (Game|GetPlayerController 0)))

(event Custom|PutDownNote
  (Widget|RemovefromParent (stale Custom|PickUpNote _returnvalue))
  (Variables|Default|SetIsReading? false))

(event Custom|TogglePickUp
  (if (Variables|Default|GetIsReading?)
    (CallFunction|PutDownNote)
    (else
      (CallFunction|PickUpNote))))

(event Custom|PickUpNote
  (bind _returnvalue (UserInterface|CreateWidget "/Game/Widgets/WBP_NoteElemental.WBP_NoteElemental_C"))
  (UserInterface|Viewport|AddtoViewport _returnvalue 0)
  (Variables|Default|SetIsReading? true))

(event EventInteract
  (params (Character :type Character%20Object%20Reference))
  (if (Variables|Default|GetInReach?)
    (CallFunction|TogglePickUp)))

(fn ConstructionScript)