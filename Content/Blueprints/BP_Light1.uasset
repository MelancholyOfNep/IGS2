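; BP_Light1 is a lamp actor that the player lights with fire damage, counting toward the lights left in the level.
; On the first damage event of a fire damage type, gated by DoOnce, it swaps the lamp mesh material to M_SnowLight1.
; It then decrements LightsLeft on BP_ThirdPersonGameMode and adds a new WBP_Lights widget to the viewport.
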(event Game|Damage|EventAnyDamage
  (params (Damage :type Float%20%28single-precision%29) (DamageType :type Damage%20Type%20Object%20Reference) (InstigatedBy :type Controller%20Object%20Reference) (DamageCauser :type Actor%20Object%20Reference))
  (if (Utilities|ClassIsChildOf (Utilities|GetClass DamageType) "/Game/Blueprints/DamageTypes/DmgTypeBP_FireDamage.DmgTypeBP_FireDamage_C")
    (Utilities|FlowControl|DoOnce false
      (:Completed
        (Rendering|Material|SetMaterial (Variables|Default|GetLampIceLevel2_pCylinder32_StaticMeshComponent0) 0 "/Game/Materials/M_SnowLight1.M_SnowLight1")
        (bind _asbp_third_person_game_mode (Utilities|Casting|CastToBP_ThirdPersonGameMode (Game|GetGameMode)))
        (bind _result (Math|Integer|DecrementInt (Variables|/Game/ThirdPerson/Blueprints/BP_ThirdPersonGameMode.BP_ThirdPersonGameMode_C|GetLightsLeft _asbp_third_person_game_mode))
          (:%20%20
            (Variables|/Game/ThirdPerson/Blueprints/BP_ThirdPersonGameMode.BP_ThirdPersonGameMode_C|SetLightsLeft _asbp_third_person_game_mode _result)
            (bind _returnvalue (UserInterface|CreateWidget "/Game/Widgets/WBP_Lights.WBP_Lights_C"))
            (UserInterface|Viewport|AddtoViewport _returnvalue 0)))))))

(fn ConstructionScript)