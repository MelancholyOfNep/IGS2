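; Slime enemy that dies when a Player-tagged actor overlaps its Box, then decrements the game mode's EnemiesLeft and shows the enemies tutorial widget.
; The height comparison meant for jump-on kills has empty branches, so any such overlap kills it.
; Capsule hits damage BP_Devvy actors with a one-second cooldown, and incoming damage drains Health until destruction.
; A looping AIMoveTo chase exists but is never started.
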(event OnComponentBeginOverlap(Box)
  (params (OverlappedComponent :type Primitive%20Component%20Object%20Reference) (OtherActor :type Actor%20Object%20Reference) (OtherComp :type Primitive%20Component%20Object%20Reference) (OtherBodyIndex :type Integer) (bFromSweep :type Boolean) (SweepResult :type Hit%20Result%20Structure%20%28by%20ref%29))
  ;[1 1 1] Enemy dies upon being jumped on
  (Development|PrintString "hit")
  (if (Actor|ActorHasTag OtherActor "Player")
    (if (< (.z (Transformation|GetWorldLocation (Variables|Character|GetMesh))) (.z (.location (Transformation|GetActorTransform (Game|GetPlayerCharacter 0)))))
      _
      (else
        _))
    (Actor|DestroyActor)
    (bind _asbp_third_person_game_mode (Utilities|Casting|CastToBP_ThirdPersonGameMode (Game|GetGameMode)))
    (bind _result (Math|Integer|DecrementInt (Variables|/Game/ThirdPerson/Blueprints/BP_ThirdPersonGameMode.BP_ThirdPersonGameMode_C|GetEnemiesLeft _asbp_third_person_game_mode))
      (:%20%20
        (Variables|/Game/ThirdPerson/Blueprints/BP_ThirdPersonGameMode.BP_ThirdPersonGameMode_C|SetEnemiesLeft _asbp_third_person_game_mode _result)
        (bind _returnvalue (UserInterface|CreateWidget "/Game/Widgets/WBP_EnemiesTutorial.WBP_EnemiesTutorial_C"))
        (UserInterface|Viewport|AddtoViewport _returnvalue 0)))))

(event OnComponentHit(CapsuleComponent)
  (params (HitComponent :type Primitive%20Component%20Object%20Reference) (OtherActor :type Actor%20Object%20Reference) (OtherComp :type Primitive%20Component%20Object%20Reference) (NormalImpulse :type Vector :default "0, 0, 0") (Hit :type Hit%20Result%20Structure%20%28by%20ref%29))
  (if (Utilities|ClassIsChildOf (Utilities|GetClass OtherActor) "/Game/NewPlayerBP/Blueprints/BP_Devvy.BP_Devvy_C")
    (if (not (Variables|Default|GetDealtDamageRecently?))
      (Variables|Default|SetDealtDamageRecently? true)
      (Game|Damage|ApplyDamage OtherActor 0.25 0 0)
      (Utilities|FlowControl|Delay 1.0)
      (Variables|Default|SetDealtDamageRecently? false))))

(event Custom|ChasePlayer
  (AI|AIMoveTo self "0, 0, 0" (Game|GetPlayerCharacter 0) 1.5e+02 false
    (:then
      (Utilities|FlowControl|Delay 2.0)
      (CallFunction|ChasePlayer))))

(event Game|Damage|EventAnyDamage
  (params (Damage :type Float%20%28single-precision%29) (DamageType :type Damage%20Type%20Object%20Reference) (InstigatedBy :type Controller%20Object%20Reference) (DamageCauser :type Actor%20Object%20Reference))
  (bind _output_get (Variables|Default|SetHealth (- (stale _output_get) Damage)))
  (if (<= _output_get 0.0)
    (Actor|DestroyActor)))

(event EventBeginPlay)

(fn ConstructionScript)