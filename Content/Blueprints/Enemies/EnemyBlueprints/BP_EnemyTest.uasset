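; Test enemy character that dies when the player jumps on it and damages BP_Devvy on contact.
; A sphere overlap destroys it if its mesh sits below the player, while capsule hits apply damage.
; A looping AIMoveTo chase is defined but never started.
; Player-style leftovers remain: a live E-key interact on overlapping actors, plus disconnected dash, power and pause-menu logic.
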(event OnComponentHit(CapsuleComponent)
  (params (HitComponent :type Primitive%20Component%20Object%20Reference) (OtherActor :type Actor%20Object%20Reference) (OtherComp :type Primitive%20Component%20Object%20Reference) (NormalImpulse :type Vector :default "0, 0, 0") (Hit :type Hit%20Result%20Structure%20%28by%20ref%29))
  (if (Utilities|ClassIsChildOf (Utilities|GetClass OtherActor) "/Game/NewPlayerBP/Blueprints/BP_Devvy.BP_Devvy_C")
    (Game|Damage|ApplyDamage OtherActor 0.25 0 0)))

(event OnComponentBeginOverlap(Sphere)
  (params (OverlappedComponent :type Primitive%20Component%20Object%20Reference) (OtherActor :type Actor%20Object%20Reference) (OtherComp :type Primitive%20Component%20Object%20Reference) (OtherBodyIndex :type Integer) (bFromSweep :type Boolean) (SweepResult :type Hit%20Result%20Structure%20%28by%20ref%29))
  ;[1 1 1] Enemy dies upon being jumped on
  (if (Components|ComponentHasTag OtherComp "Player")
    (if (< (.z (Transformation|GetWorldLocation (Variables|Character|GetMesh))) (.z (.location (Transformation|GetActorTransform (Game|GetPlayerCharacter 0)))))
      (Actor|DestroyActor))))

(event Custom|ChasePlayer
  (AI|AIMoveTo self "0, 0, 0" (Game|GetPlayerCharacter 0) 1.5e+02 false
    (:then
      (Utilities|FlowControl|Delay 2.0)
      (CallFunction|ChasePlayer))))

(event Input|EnhancedActionEvents|EnhancedInputActionIA_Power
  (params (ActionValue :type Boolean) (ElapsedSeconds :type Float%20%28double-precision%29) (TriggeredSeconds :type Float%20%28double-precision%29) (InputAction :type Input%20Action%20Object%20Reference :default "/Game/ThirdPerson/Input/Actions/IA_Power.IA_Power")))

(event Input|EnhancedActionEvents|EnhancedInputActionIA_Dash
  (params (ActionValue :type Boolean) (ElapsedSeconds :type Float%20%28double-precision%29) (TriggeredSeconds :type Float%20%28double-precision%29) (InputAction :type Input%20Action%20Object%20Reference :default "/Game/ThirdPerson/Input/Actions/IA_Dash.IA_Dash")))

(event EventBeginPlay)

(event Input|KeyboardEvents|E
  (params (Key :type Key%20Structure :default "None"))
  (:Pressed
    (bind _array_element (Utilities|Array|ForEachLoopwithBreak (Collision|GetOverlappingActors "/Script/Engine.Actor" :!class /Script/Engine.Actor) :!label _label)
      (:LoopBody
        (if (Utilities|DoesObjectImplementInterface _array_element "/Game/Blueprints/BPI_Interact.BPI_Interact_C")
          (Class|BPIInteract|Interact(Message) _array_element)
          (goto _label Break))))))

(fn ConstructionScript)