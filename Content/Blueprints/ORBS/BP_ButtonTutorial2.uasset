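; Tutorial button actor that opens the BP_WoodDoor matching its ButtonValue once the game mode reports no enemies left.
; Box overlap toggles the prompt widget and the actor's input.
; Interact runs the opening once: it disables character input, pauses enemy and cave AI via blackboard bools, and blends the camera to the door, restoring control and AI five seconds later.
; With enemies remaining, Interact shows WBP_EnemiesFail instead.
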(event OnComponentBeginOverlap(Box)
  (params (OverlappedComponent :type Primitive%20Component%20Object%20Reference) (OtherActor :type Actor%20Object%20Reference) (OtherComp :type Primitive%20Component%20Object%20Reference) (OtherBodyIndex :type Integer) (bFromSweep :type Boolean) (SweepResult :type Hit%20Result%20Structure%20%28by%20ref%29))
  ;[1 1 1] Widget
  (Rendering|SetVisibility (Variables|Default|GetWidget) true false)
  (Input|EnableInput (Game|GetPlayerController 0)))

(event OnComponentEndOverlap(Box)
  (params (OverlappedComponent :type Primitive%20Component%20Object%20Reference) (OtherActor :type Actor%20Object%20Reference) (OtherComp :type Primitive%20Component%20Object%20Reference) (OtherBodyIndex :type Integer))
  ;[1 1 1] Widget
  (Rendering|SetVisibility (Variables|Default|GetWidget) false false)
  (Input|DisableInput (Game|GetPlayerController 0)))

(event Input|EnhancedActionEvents|EnhancedInputActionIA_Interact
  (params (ActionValue :type Boolean) (ElapsedSeconds :type Float%20%28double-precision%29) (TriggeredSeconds :type Float%20%28double-precision%29) (InputAction :type Input%20Action%20Object%20Reference :default "/Game/ThirdPerson/Input/Actions/IA_Interact.IA_Interact")))

(event EventInteract
  (params (Character :type Character%20Object%20Reference))
  (bind _returnvalue (Game|GetPlayerController 0))
  (bind _asbp_third_person_game_mode (Utilities|Casting|CastToBP_ThirdPersonGameMode (Game|GetGameMode)))
  (if (== (Variables|/Game/ThirdPerson/Blueprints/BP_ThirdPersonGameMode.BP_ThirdPersonGameMode_C|GetEnemiesLeft _asbp_third_person_game_mode) 0)
    (bind _outactors (Actor|GetAllActorsOfClass "/Game/Blueprints/BP_WoodDoor.BP_WoodDoor_C"))
    (bind _array_element (Utilities|Array|ForEachLoopwithBreak _outactors)
      (:LoopBody
        (if (== (Variables|/Game/Blueprints/BP_WoodDoor.BP_WoodDoor_C|GetDoorValue _array_element) (Variables|Default|GetButtonValue))
          (Utilities|FlowControl|DoOnce false
            (:Completed
              (Utilities|FlowControl|Sequence
                (:then_0
                  (Input|DisableInput Character _returnvalue)
                  (CallFunction|AIPause)
                  (Default|OpenDoor _array_element Character)
                  (Game|Player|SetViewTargetwithBlend _returnvalue _array_element 0.0 "VTBlend_Linear" 0.0 false)
                  (Utilities|FlowControl|Delay 5.0)
                  (Input|EnableInput Character (Game|GetPlayerController 0))
                  (CallFunction|AIUnpause))
                (:then_1
                  (Rendering|SetVisibility (Variables|Default|GetWidget) false false)
                  (Input|DisableInput (Game|GetPlayerController 0)))))))))
    (else
      (bind _returnvalue_2 (UserInterface|CreateWidget "/Game/Widgets/WBP_EnemiesFail.WBP_EnemiesFail_C"))
      (UserInterface|Viewport|AddtoViewport _returnvalue_2 0))))

(event Input|KeyboardEvents|E
  (params (Key :type Key%20Structure :default "None")))

(fn ConstructionScript)

(fn AIPause
  (bind _outactors (Actor|GetAllActorsOfClass "/Game/Blueprints/Enemies/EnemyBlueprints/BP_EnemyController.BP_EnemyController_C"))
  (for _array_element _outactors
    (AI|Components|Blackboard|SetValueasBool (AI|GetBlackboard _array_element) (Utilities|Name|MakeLiteralName "AIPause") true))
  (bind _outactors_2 (Actor|GetAllActorsOfClass "/Game/Blueprints/Enemies/EnemyBlueprints/BP_CaveController.BP_CaveController_C"))
  (for _array_element_2 _outactors_2
    (AI|Components|Blackboard|SetValueasBool (AI|GetBlackboard _array_element_2) (Utilities|Name|MakeLiteralName "AIPause") true))
  (return))

(fn AIUnpause
  (bind _outactors (Actor|GetAllActorsOfClass "/Game/Blueprints/Enemies/EnemyBlueprints/BP_EnemyController.BP_EnemyController_C"))
  (for _array_element _outactors
    (AI|Components|Blackboard|SetValueasBool (AI|GetBlackboard _array_element) (Utilities|Name|MakeLiteralName "AIPause") false))
  (bind _outactors_2 (Actor|GetAllActorsOfClass "/Game/Blueprints/Enemies/EnemyBlueprints/BP_CaveController.BP_CaveController_C"))
  (for _array_element_2 _outactors_2
    (AI|Components|Blackboard|SetValueasBool (AI|GetBlackboard _array_element_2) (Utilities|Name|MakeLiteralName "AIPause") false))
  (return))