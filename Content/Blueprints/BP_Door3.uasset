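; BP_Door3 is a door that slides its static mesh downward when its OpenDoor event is called with a player.
; A timeline drives the vertical lerp, while input is disabled if the player is a BP_Devvy.
; When the timeline finishes, a short delay precedes blending the view target back to the player and re-enabling their input.
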(event Custom|OpenDoor
  (params (Player :type Actor%20Object%20Reference))
  (Utilities|FlowControl|Sequence
    (:then_0
      (bind _newtrack_0 (Timeline|OpenDoor1 Play)
        (:Update
          (Transformation|SetRelativeLocation (Variables|Default|GetStaticMesh) (Math|Vector|Lerp(Vector) "0, 0, 0" "0.000000,0.000000,-3700.000000" _newtrack_0) false false))
        (:Finished
          (Utilities|FlowControl|Delay 1.0)
          (Game|Player|SetViewTargetwithBlend (Game|GetPlayerController 0) Player 1.0 "VTBlend_Linear" 0.0 false)
          (Input|EnableInput Player 0))))
    (:then_1
      (bind _asbp_devvy (Utilities|Casting|CastToBP_Devvy Player))
      (Input|DisableInput _asbp_devvy 0))))

(fn ConstructionScript)