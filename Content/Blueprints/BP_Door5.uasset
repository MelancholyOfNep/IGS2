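; BP_Door5 is an interactable door that opens only once the LightsLeft count in BP_ThirdPersonGameMode reaches zero.
; Overlapping its Box shows a Widget component and enables player input on the door; leaving reverses both.
; Pressing E either plays a timeline that lerps the mesh downward, or shows a fail widget followed by a delayed hint widget.
; The OpenSecretDoor function is an empty stub.
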(event OnComponentBeginOverlap(Box)
  (params (OverlappedComponent :type Primitive%20Component%20Object%20Reference) (OtherActor :type Actor%20Object%20Reference) (OtherComp :type Primitive%20Component%20Object%20Reference) (OtherBodyIndex :type Integer) (bFromSweep :type Boolean) (SweepResult :type Hit%20Result%20Structure%20%28by%20ref%29))
  ;[1 1 1] Widget
  (Rendering|SetVisibility (Variables|Default|GetWidget) true false)
  (Input|EnableInput (Game|GetPlayerController 0)))

(event OnComponentEndOverlap(Box)
  (params (OverlappedComponent :type Primitive%20Component%20Object%20Reference) (OtherActor :type Actor%20Object%20Reference) (OtherComp :type Primitive%20Component%20Object%20Reference) (OtherBodyIndex :type Integer))
  ;[1 1 1] Widget
  (Rendering|SetVisibility (Variables|Default|GetWidget) false false)
  (Input|DisableInput (Game|GetPlayerController 0)))

(event Input|KeyboardEvents|E
  (params (Key :type Key%20Structure :default "None"))
  (:Pressed
    (bind _asbp_third_person_game_mode (Utilities|Casting|CastToBP_ThirdPersonGameMode (Game|GetGameMode)))
    (if (== (Variables|/Game/ThirdPerson/Blueprints/BP_ThirdPersonGameMode.BP_ThirdPersonGameMode_C|GetLightsLeft _asbp_third_person_game_mode) 0)
      (bind _newtrack_0 (Timeline|OpenDoor1 Play)
        (:Update
          (Transformation|SetRelativeLocation (Variables|Default|GetStaticMesh) (Math|Vector|Lerp(Vector) "0, 0, 0" "0.000000,0.000000,-1000.000000" _newtrack_0) false false)))
      (else
        (bind _returnvalue (UserInterface|CreateWidget "/Game/Widgets/WBP_LightsFail.WBP_LightsFail_C"))
        (UserInterface|Viewport|AddtoViewport _returnvalue 0)
        (Utilities|FlowControl|Delay 4.0)
        (bind _returnvalue_2 (UserInterface|CreateWidget "/Game/Widgets/WBP_LightsHint.WBP_LightsHint_C"))
        (UserInterface|Viewport|AddtoViewport _returnvalue_2 0)))))

(fn ConstructionScript)

(fn OpenSecretDoor
  (params (Player :type Actor%20Object%20Reference)))