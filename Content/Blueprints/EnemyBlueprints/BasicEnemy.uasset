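; Basic enemy that damages the player character class BP_UITest on contact and dies when jumped on.
; A sphere overlap destroys the enemy if player 0 is higher than its cylinder, without checking which actor overlapped.
; Cylinder hits apply a small amount of damage to BP_UITest actors, throttled by a DealtDamageRecently flag that resets after a one-second delay.
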(event OnComponentBeginOverlap(Sphere)
  (params (OverlappedComponent :type Primitive%20Component%20Object%20Reference) (OtherActor :type Actor%20Object%20Reference) (OtherComp :type Primitive%20Component%20Object%20Reference) (OtherBodyIndex :type Integer) (bFromSweep :type Boolean) (SweepResult :type Hit%20Result%20Structure%20%28by%20ref%29))
  ;[1 1 1] Enemy dies upon being jumped on
  (if (< (.z (Transformation|GetWorldLocation (Variables|Default|GetCylinder))) (.z (.location (Transformation|GetActorTransform (Game|GetPlayerCharacter 0)))))
    (Actor|DestroyActor)))

(event OnComponentHit(Cylinder)
  (params (HitComponent :type Primitive%20Component%20Object%20Reference) (OtherActor :type Actor%20Object%20Reference) (OtherComp :type Primitive%20Component%20Object%20Reference) (NormalImpulse :type Vector :default "0, 0, 0") (Hit :type Hit%20Result%20Structure%20%28by%20ref%29))
  (if (Utilities|ClassIsChildOf (Utilities|GetClass OtherActor) "/Game/ThirdPerson/Blueprints/BP_UITest.BP_UITest_C")
    (if (not (Variables|Default|GetDealtDamageRecently?))
      (Game|Damage|ApplyDamage OtherActor 0.25 0 0)
      (Variables|Default|SetDealtDamageRecently? true)
      (Utilities|FlowControl|Delay 1.0)
      (Variables|Default|SetDealtDamageRecently? false))))

(event EventBeginPlay)

(event EventTick
  (params (DeltaSeconds :type Float%20%28single-precision%29)))

(fn ConstructionScript)