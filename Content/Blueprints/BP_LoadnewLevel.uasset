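; BP_LoadnewLevel is an overlap trigger that moves the BP_Devvy player into a newly streamed level.
; On overlap it disables input, shows the LoadingScreen1 widget, starts a non-blocking load of LevelToLoad and immediately moves the player to its Capsule component's location.
; A fixed six-second delay, rather than a load-completion callback, hides the transition before it removes the widget, restores input and unloads CurrentLevel.
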(event EventBeginPlay)

(event Collision|EventActorBeginOverlap
  (params (OtherActor :type Actor%20Object%20Reference))
  (bind _asbp_devvy (Utilities|Casting|CastToBP_Devvy OtherActor))
  (Input|DisableInput _asbp_devvy (Game|GetPlayerController 0))
  (bind _returnvalue (UserInterface|CreateWidget "/Game/Movies/LoadingScreen1.LoadingScreen1_C"))
  (UserInterface|Viewport|AddtoViewport _returnvalue 0)
  (Class|GameplayStatics|LoadStreamLevelbySoftObjectPtr (Variables|Default|GetLevelToLoad) true false)
  (Transformation|SetActorLocation _asbp_devvy (Transformation|GetWorldLocation (Variables|Default|GetCapsule)) false false)
  (Utilities|FlowControl|Delay 6.0)
  (Widget|RemovefromParent _returnvalue)
  (Input|EnableInput _asbp_devvy (Game|GetPlayerController 0))
  (Class|GameplayStatics|UnloadStreamLevelbySoftObjectPtr (Variables|Default|GetCurrentLevel) false))

(event EventTick
  (params (DeltaSeconds :type Float%20%28single-precision%29)))

(fn ConstructionScript)