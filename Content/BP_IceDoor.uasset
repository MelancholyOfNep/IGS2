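; BP_IceDoor is an ice door actor that is destroyed by fire damage or by interaction once power is picked up.
; PickUpPower sets HasPower, letting Interact alternate WallTimeline between play and reverse through a FlipFlop.
; The timeline's Update destroys the actor, while a mesh yaw rotation driven by the timeline track is left disconnected.
; AnyDamage destroys the door when the damage type is a child of DmgTypeBP_FireDamage.
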(event EventInteract
  (if (Variables|Default|GetHasPower?)
    (Utilities|FlowControl|FlipFlop
      (:A
        (bind _walltrack (Timeline|Wall%20Timeline Play)
          (:Update
            (Actor|DestroyActor))))
      (:B
        (Timeline|Wall%20Timeline Reverse)))))

(event EventPickUpPower
  (Variables|Default|SetHasPower? true))

(event Game|Damage|EventAnyDamage
  (params (Damage :type Float%20%28single-precision%29) (DamageType :type Damage%20Type%20Object%20Reference) (InstigatedBy :type Controller%20Object%20Reference) (DamageCauser :type Actor%20Object%20Reference))
  (if (Utilities|ClassIsChildOf (Utilities|GetClass DamageType) "/Game/Blueprints/DamageTypes/DmgTypeBP_FireDamage.DmgTypeBP_FireDamage_C")
    (Actor|DestroyActor)))

(fn ConstructionScript)