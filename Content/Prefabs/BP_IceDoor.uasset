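; BP_IceDoor is an ice door that only fire damage removes.
; A fire damage type plays a timeline that slides the mesh down along Z, and a two-second delay started from its update destroys the actor.
; Box overlap shows or hides a widget and toggles player input.
; Interact is empty, and a power-gated rotating door timeline is left unconnected, so the HasPower flag has no live effect.
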(event OnComponentBeginOverlap(Box)
  (params (OverlappedComponent :type Primitive%20Component%20Object%20Reference) (OtherActor :type Actor%20Object%20Reference) (OtherComp :type Primitive%20Component%20Object%20Reference) (OtherBodyIndex :type Integer) (bFromSweep :type Boolean) (SweepResult :type Hit%20Result%20Structure%20%28by%20ref%29))
  ;[1 1 1] Widget
  (Rendering|SetVisibility (Variables|Default|GetWidget) true false)
  (Input|EnableInput (Game|GetPlayerController 0)))

(event OnComponentEndOverlap(Box)
  (params (OverlappedComponent :type Primitive%20Component%20Object%20Reference) (OtherActor :type Actor%20Object%20Reference) (OtherComp :type Primitive%20Component%20Object%20Reference) (OtherBodyIndex :type Integer))
  ;[1 1 1] Widget
  (Rendering|SetVisibility (Variables|Default|GetWidget) false false)
  (Input|DisableInput (Game|GetPlayerController 0)))

(event EventInteract
  (params (Character :type Character%20Object%20Reference)))

(event EventPickUpPower
  (Variables|Default|SetHasPower? true))

(event Game|Damage|EventAnyDamage
  (params (Damage :type Float%20%28single-precision%29) (DamageType :type Damage%20Type%20Object%20Reference) (InstigatedBy :type Controller%20Object%20Reference) (DamageCauser :type Actor%20Object%20Reference))
  (if (Utilities|ClassIsChildOf (Utilities|GetClass DamageType) "/Game/Blueprints/DamageTypes/DmgTypeBP_FireDamage.DmgTypeBP_FireDamage_C")
    (bind _newtrack_0 (Timeline|Timeline Play)
      (:Update
        (Transformation|SetRelativeLocation (Variables|Default|GetStaticMesh) (Math|Vector|Lerp(Vector) "0.000000,0.000000,-220.000000" "0.000000,0.000000,-974.000000" _newtrack_0) false false)
        (Utilities|FlowControl|Delay 2.0)
        (Actor|DestroyActor)))))

(fn ConstructionScript)